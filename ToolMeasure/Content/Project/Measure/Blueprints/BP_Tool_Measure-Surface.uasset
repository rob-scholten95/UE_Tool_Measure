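; Surface measuring tool that lets the player outline a four-point area with the mouse and calculates its area.
; A closed spline's unlocked points follow the cursor's floor hit, and each left click locks the next point, resetting once all are placed.
; Looping timers drive updates, with spline meshes drawing edges and small static meshes marking corners.
; Segment lengths feed an irregular-quadrilateral area calculation, with optional debug display of lengths, indices, area, midpoint and angles.
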(event Custom|DebugSpline
  (bind _spline (Variables|Default|GetSpline))
  ;[1 1 1] Debug Functions
  (CallFunction|DebugShowSegmentLengthsonSpline (Variables|Default|GetSegment%20Lengths) (Variables|Default|GetSpline) "NewEnumerator0")
  (CallFunction|DebugShowIndicesonSpline (Variables|Default|GetSpline))
  (CallFunction|DebugShowAreaonSpline (Variables|Default|GetSpline) (Variables|Default|GetTotalArea) "NewEnumerator6")
  (CallFunction|DebugShowMidpointonSpline _spline 5e+01)
  (CallFunction|DebugShowAngles _spline))

(event Custom|UpdateSplineActiveSplinePoint
  ;[1 1 1] Comment
  (for _array_element (Variables|Default|GetPointsToControl)
    (Spline|SetLocationatSplinePoint (Variables|Default|GetSpline) _array_element (Tracing|GetHitLocationMouseonFloor) "Local" true)))

(event Custom|UpdateLineVisuals
  (bind _spline (Variables|Default|GetSpline))
  ;[1 1 1] Comment
  (Utilities|FlowControl|Sequence
    (:then_0
      (for (_array_element _array_index) (Variables|Default|GetSplineMeshComponent)
        (SplineMesh|SetStartandEnd _array_element (.Location (Spline|GetLocationandTangentatSplinePoint _spline _array_index "Local")) (.Tangent (Spline|GetLocationandTangentatSplinePoint _spline _array_index "Local")) (.Location (Spline|GetLocationandTangentatSplinePoint _spline (+ _array_index 1) "Local")) (.Tangent (Spline|GetLocationandTangentatSplinePoint _spline (+ _array_index 1) "Local")) true :!class /Script/Engine.SplineMeshComponent)))
    (:then_1
      (for (_array_element_2 _array_index_2) (Variables|Default|GetMeshComponents)
        (Transformation|SetWorldLocation _array_element_2 (.Location (Spline|GetLocationandTangentatSplinePoint (Variables|Default|GetSpline) _array_index_2 "Local")) false false)))))

(event Custom|CalculateSplineArea
  ;[1 1 1] Calculate Spline Area
  (bind _segment_lengths (CallFunction|GetAllSplineSegmentsLengths (Variables|Default|GetSpline)))
  (bind _output_get (Variables|Default|SetSegment%20Lengths _segment_lengths))
  (bind _keys (Utilities|Map|Keys _output_get))
  (bind _output_get_2 (Variables|Default|SetSegmentLengths _keys))
  (bind _area_in_m2 (CallFunction|CalculateAreaOfIrregularQuadrilateral (Variables|Default|GetSpline) _output_get_2))
  (Variables|Default|SetTotalArea _area_in_m2))

(event EventBeginPlay
  ;[1 1 1] ON BEGINPLAY
  (Utilities|FlowControl|Sequence
    (:then_0
      (CallFunction|ResetArray))
    (:then_1
      (|InitializeSpline))
    (:then_2
      (Utilities|Time|SetTimerbyEvent (EventDispatchers|CreateEvent :!event Custom|UpdateSplineActiveSplinePoint) 0.01 true))
    (:then_3
      (|CreatingVisualElementsoftheSpline))
    (:then_4
      (|StartDebugSplineFunctions))
    (:then_5
      (Utilities|Time|SetTimerbyEvent (EventDispatchers|CreateEvent :!event Custom|CalculateSplineArea) 0.01 true))))

(fn ConstructionScript)

(fn GetHitLocationMouseonFloor
  (bind _returnvalue (Game|GetPlayerController 0))
  (bind _hitresult (Game|Player|GetHitResultUnderCursorbyChannel _returnvalue "TraceTypeQuery1" false))
  (bind (_bblockinghit _binitialoverlap _time _distance _location) (Collision|BreakHitResult _hitresult))
  (if _bblockinghit
    (return _location)
    (else
      (return "0.000000,0.000000,-50000.000000"))))

(fn ResetArray
  (Variables|Default|SetPointsToControl (Utilities|Array|MakeArray 0 1 2 3)))

(fn OnLeftMouseClick
  (if (Utilities|Array|IsEmpty (Variables|Default|GetPointsToControl))
    (CallFunction|ResetArray)
    (else
      (Utilities|Array|RemoveIndex (Variables|Default|GetPointsToControl)))))