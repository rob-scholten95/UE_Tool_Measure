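; Measurement tool manager actor that lets the player run linear or surface measurements through an on-screen button widget.
; On BeginPlay it enables mouse input, creates the buttons and a cursor icon widget, which a looping timer keeps on the mouse.
; EnableMeasureType spawns the chosen measure-type actor, or only destroys the active one if present.
; Left clicks forward to that actor, and destroying the tool removes it and both widgets.
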(event Custom|UpdateCursorImageLocation
  ;[0 1 0.01552] MeasureIconOnCursor
  ;;[1 0 0.7451] Timed Event - Update Cursor image based on the mouse position
  (bind _returnvalue (Class|WidgetLayoutLibrary|GetMousePositiononViewport))
  (Class|UserWidget|SetPositioninViewport (Variables|Widgets|GetCursorImageWidget) _returnvalue false))

(event Input|EnhancedActionEvents|EnhancedInputActionIA_MouseLeftClick
  (params (ActionValue :type Boolean) (ElapsedSeconds :type Float%20%28double-precision%29) (TriggeredSeconds :type Float%20%28double-precision%29) (InputAction :type Input%20Action%20Object%20Reference :default "/Game/Project/Measure/Input/IA_MouseLeftClick.IA_MouseLeftClick"))
  (bind _measuretypeactor (Variables|Measure|GetMeasureTypeActor))
  ;[0 1 0.01552] Input Handler
  (:Started
    (Utilities|IsValid _measuretypeactor
      (:Is%20Valid
        (Default|OnLeftMouseClick _measuretypeactor)))))

(event EventBeginPlay
  (bind _returnvalue (Game|GetPlayerController 0))
  (Utilities|FlowControl|Sequence
    (:then_0
      ;[1 0 0] CAN BE IMPLEMENTED IN YOUR OWN PLAYERCONTROLLER
      (Variables|/Script/Engine.PlayerController|SetbShowMouseCursor _returnvalue true)
      (Input|SetInputModeGameandUI _returnvalue 0 "DoNotLock" true false))
    (:then_1
      ;[1 0 0] CAN BE IMPLEMENTED IN YOUR OWN PLAYERCONTROLLER
      (Input|AddMappingContext (PlayerController|LocalPlayerSubsystems|GetEnhancedInputLocalPlayerSubsystem (Game|GetPlayerController 0)) "/Game/Project/Measure/Input/IMC_Click.IMC_Click" 0 "(bIgnoreAllPressedKeysUntilRelease=True,bForceImmediately=False,bNotifyUserSettings=False)"))
    (:then_2
      ;[0 1 0.01552] Creating Button Widget
      (bind _returnvalue_2 (UserInterface|CreateWidget "/Game/Project/Measure/Widgets/UW_Buttons.UW_Buttons_C" 0 self))
      (bind _output_get (Variables|Widgets|SetButtonsWidget _returnvalue_2))
      (UserInterface|Viewport|AddtoViewport _output_get 0))
    (:then_3
      ;[0 1 0.01552] MeasureIconOnCursor
      ;;[1 1 1] Create Cursor Image
      (bind _returnvalue_3 (UserInterface|CreateWidget "/Game/Project/Measure/Widgets/UW_CursorImage.UW_CursorImage_C"))
      (bind _output_get_2 (Variables|Widgets|SetCursorImageWidget _returnvalue_3))
      (Variables|/Game/Project/Measure/Widgets/UW_CursorImage.UW_CursorImage_C|SetCursorIcon _output_get_2 (Variables|Default|GetCursor%20Icon))
      ;;[1 1 1] Start Updating Cursor Location
      (Utilities|Time|SetTimerbyEvent (EventDispatchers|CreateEvent :!event Custom|UpdateCursorImageLocation) 0.01 true)
      (UserInterface|Viewport|AddtoViewport _output_get_2 0))))

(event EventDestroyed
  (bind _measuretypeactor (Variables|Measure|GetMeasureTypeActor))
  ;[0 1 0.01552] Exit Measure Mode
  (Widget|RemovefromParent (Variables|Widgets|GetCursorImageWidget))
  (Utilities|IsValid _measuretypeactor
    (:Is%20Valid
      (Actor|DestroyActor _measuretypeactor))))

(fn ConstructionScript)

(fn EnableMeasureType
  (params (MeasureTypes :type E_MeasureTypes%20Enum :default "NewEnumerator0"))
  (bind _output_get (Variables|Measure|SetMeasureType MeasureTypes))
  (if (not (Utilities|Enum|Equal(Enum) _output_get "NewEnumerator0"))
    (bind _measuretypeactor (Variables|Measure|GetMeasureTypeActor)
      (:then
        (Actor|DestroyActor _measuretypeactor :!label _label)
        (Variables|Measure|SetMeasureTypeActor 0))
      (:else
        (bind _returnvalue (Game|SpawnActorfromClass (Utilities|Select :Index _output_get :NewEnumerator0 0 :NewEnumerator1 "/Game/Project/Measure/Blueprints/BP_Tool_Measure-Surface.BP_Tool_Measure-Surface_C" :NewEnumerator3 "/Game/Project/Measure/Blueprints/BP_Tool_Measure-Linear.BP_Tool_Measure-Linear_C") (Math|Transform|MakeTransform "0, 0, 0" "0, 0, 0" "1.000000,1.000000,1.000000") "Undefined" "MultiplyWithRoot" 0 0))
        (bind _asbp_tool_measure__type (Utilities|Casting|CastToBP_Tool_Measure-Type _returnvalue))
        (Variables|Measure|SetMeasureTypeActor _asbp_tool_measure__type)))
    (else
      (goto _label))))