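; Linear measure tool that draws a line between two cursor-placed points and shows its length at the midpoint.
; Fast looping timers, rather than Tick, move unpinned spline points to the cursor's Visibility trace hit and refresh the spline mesh, endpoint markers and unit-converted distance widget.
; Left clicks pin the points in turn via the PointsToControl array, then restart once both are set; right click resets both.
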(event Custom|UpdateSplineActiveSplinePoint
  ;[1 0 0] TIMED EVENTS
  ;;[1 0.6564 0.5998] Comment
  (for _array_element (Variables|Default|GetPointsToControl)
    (Spline|SetLocationatSplinePoint (Variables|Default|GetSpline) _array_element (CallFunction|GetHitLocationMouseonFloor) "Local" true)))

(event Custom|UpdateDistanceText
  (bind _spline (Variables|Default|GetSpline))
  ;[1 0 0] TIMED EVENTS
  ;;[1 0.6564 0.5998] Comment
  (Default|SetDistanceText (Variables|Default|GetDistanceText) (CallFunction|ConvertValuetoUnit (Variables|Default|GetUnit) (Spline|GetSplineLength (Variables|Default|GetSpline))))
  (Transformation|SetWorldLocation (Variables|Default|GetWidget) (CallFunction|GetSplineMidpoint (Spline|GetLocationatSplinePoint _spline 0 "Local") (Spline|GetLocationatSplinePoint _spline 1 "Local")) false false))

(event Custom|UpdateLineVisuals
  (bind _spline (Variables|Default|GetSpline))
  (bind _spline_2 (Variables|Default|GetSpline))
  (bind (_location _tangent) (Spline|GetLocationandTangentatSplinePoint _spline_2 1 "Local"))
  (bind (_location_2 _tangent_2) (Spline|GetLocationandTangentatSplinePoint _spline_2 0 "Local"))
  ;[1 0 0] TIMED EVENTS
  ;;[1 1 1] Comment
  (Utilities|FlowControl|Sequence
    (:then_0
      (SplineMesh|SetStartandEnd (Variables|Default|GetSplineMesh) _location_2 _tangent_2 _location _tangent true :!class /Script/Engine.SplineMeshComponent))
    (:then_1
      ;;[1 1 1] Comment
      (Transformation|SetWorldLocation (Variables|Default|GetPoint1) (Spline|GetLocationatSplinePoint _spline 0 "World") false false)
      (Transformation|SetWorldLocation (Variables|Default|GetPoint2) (Spline|GetLocationatSplinePoint _spline 1 "World") false false))))

(event EventBeginPlay
  (bind _splinemesh (Variables|Default|GetSplineMesh))
  (bind _linewidth (Variables|Default|GetLineWidth))
  (bind _returnvalue (Math|Conversions|ToVector2D(Vector) _linewidth))
  ;[0.5666 0.5465 1] ON BEGINPLAY
  (Utilities|FlowControl|Sequence
    (:then_0
      ;;[1 1 1] Comment
      (Variables|Default|SetPointsToControl (Utilities|Array|MakeArray 0 1))
      (Utilities|Time|SetTimerbyEvent (EventDispatchers|CreateEvent :!event Custom|UpdateSplineActiveSplinePoint) 0.01 true))
    (:then_1
      ;;[1 1 1] Comment
      (bind _asuw_distance_text (Utilities|Casting|CastToUW_DistanceText (UserInterface|GetWidget (Variables|Default|GetWidget))))
      (bind _output_get (Variables|Default|SetDistanceText _asuw_distance_text))
      (Default|SetDistanceText _output_get)
      (bind _returnvalue_2 (Utilities|Time|SetTimerbyEvent (EventDispatchers|CreateEvent :!event Custom|UpdateDistanceText) 0.01 true))
      (Variables|Default|SetTimer_DistanceText _returnvalue_2))
    (:then_2
      ;;[1 1 1] Comment
      (SplineMesh|SetEndScale _splinemesh _returnvalue true :!class /Script/Engine.SplineMeshComponent)
      (SplineMesh|SetStartScale _splinemesh _returnvalue true :!class /Script/Engine.SplineMeshComponent))
    (:then_3
      ;;[1 1 1] Comment
      (Utilities|Time|SetTimerbyEvent (EventDispatchers|CreateEvent :!event Custom|UpdateLineVisuals) 0.01 true))))

(fn ConstructionScript)

(fn GetHitLocationMouseonFloor
  (bind _returnvalue (Game|GetPlayerController 0))
  (bind _hitresult (Game|Player|GetHitResultUnderCursorbyChannel _returnvalue "TraceTypeQuery1" false))
  (bind (_bblockinghit _binitialoverlap _time _distance _location) (Collision|BreakHitResult _hitresult))
  (if _bblockinghit
    (return _location)
    (else
      (return "0.000000,0.000000,-50000.000000"))))

(fn OnLeftMouseClick
  (if (Utilities|Array|IsEmpty (Variables|Default|GetPointsToControl))
    (Variables|Default|SetPointsToControl (Utilities|Array|MakeArray 0 1))
    (bind _returnvalue (Utilities|Time|SetTimerbyEvent (EventDispatchers|CreateEvent :!event Custom|UpdateDistanceText) 0.01 true))
    (Variables|Default|SetTimer_DistanceText _returnvalue)
    (else
      (Utilities|Array|RemoveIndex (Variables|Default|GetPointsToControl))
      (if (== (Utilities|Array|Length (Variables|Default|GetPointsToControl)) 0)
        (Utilities|Time|ClearandInvalidateTimerbyHandle (Variables|Default|GetTimer_DistanceText))))))

(fn GetSplineMidpoint
  (params (Vector%201 :type Vector) (Vector%202 :type Vector))
  (bind (_x _y _z) (Math|Vector|BreakVector Vector%201))
  (bind (_x_2 _y_2 _z_2) (Math|Vector|BreakVector Vector%202))
  (return (Math|Vector|MakeVector (/ (+ _x _x_2) 2.0) (/ (+ _y _y_2) 2.0) (/ (+ _z _z_2) 2.0))))

(fn OnRightMouseClick
  (Variables|Default|SetPointsToControl (Utilities|Array|MakeArray 0 1))
  (bind _returnvalue (Utilities|Time|SetTimerbyEvent (EventDispatchers|CreateEvent :!event Custom|UpdateDistanceText) 0.01 true))
  (Variables|Default|SetTimer_DistanceText _returnvalue))